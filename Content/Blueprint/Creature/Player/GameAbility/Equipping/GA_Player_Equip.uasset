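; Gameplay ability that equips the player's carried weapon, selected by weapon tag.
; It plays an equip montage and, on the equip gameplay event, snaps the weapon to its socket and records it as the current equipped weapon.
; From the weapon's data it links the anim layer, adds the input mapping context, grants weapon abilities and updates weapon and ability UI, including running cooldowns.
; The ability ends when the montage finishes or is interrupted.
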(event Ability|EventActivateAbility
  (|PlayMontageandWaitProxy "None" (Variables|Default|GetMontage%20to%20Play) 1.0 "None" true 1.0 0.0 false
    (:then
      (Ability|Tasks|WaitGameplayEvent "(TagName=\"Player.Event.Equip.Axe\")" 0
        (:EventReceived
          (Transformation|AttachComponentToComponent (Class|CPawnCombatComponent|GetCreatureCarriedWeaponbyTag (Class|CPlayerGameplayAbility|GetPlayerCombatComponentfromActorInfo) (Variables|Default|GetPlayerWeaponTag)) (Class|GameplayAbility|GetOwningComponentfromActorInfo) (.EquipSocketName (Utilities|Struct|BreakPlayerWeaponData (Variables|/Script/ABD_RPGSystem.C_PlayerWeapon|GetPlayerWeaponData (Class|CPlayerCombatComponent|GetPlayerCarriedWeaponbyTag (Class|CPlayerGameplayAbility|GetPlayerCombatComponentfromActorInfo) (Variables|Default|GetPlayerWeaponTag))))) "SnapToTarget" "KeepRelative" "KeepWorld" true)
          (CallFunction|HandleEquipWeapon (Class|CPlayerCombatComponent|GetPlayerCarriedWeaponbyTag (Class|CPlayerGameplayAbility|GetPlayerCombatComponentfromActorInfo) (Variables|Default|GetPlayerWeaponTag)))
          (Variables|/Script/ABD_RPGSystem.C_PawnCombatComponent|SetCurrentEquippedWeaponTag (Class|CPlayerGameplayAbility|GetPlayerCombatComponentfromActorInfo) (Variables|Default|GetPlayerWeaponTag)))))
    (:OnCompleted
      (Ability|EndAbility :!label _label))
    (:OnBlendOut
      (goto _label))
    (:OnInterrupted
      (goto _label))
    (:OnCancelled
      (goto _label))))

(event Ability|EventOnEndAbility
  (params (bWasCancelled :type Boolean)))

(fn HandleEquipWeapon
  (params (InEquipWeapon :type C%20Player%20Weapon%20Object%20Reference))
  (LocalVariables|SetCachedWeaponData (Variables|/Script/ABD_RPGSystem.C_PlayerWeapon|GetPlayerWeaponData InEquipWeapon))
  (Utilities|FlowControl|Sequence
    (:then_0
      (|ChageAnimLayer))
    (:then_1
      (|BindInput))
    (:then_2
      (|GiveAbilitytoActor))
    (:then_3
      (|UpdateUI))))