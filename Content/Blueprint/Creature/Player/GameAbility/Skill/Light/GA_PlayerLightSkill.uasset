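; GA_PlayerLightSkill is the player's light special weapon skill, a gameplay ability that plays an attack montage and ends when the montage finishes or is interrupted.
; While it plays, melee-hit events apply weapon-based damage tagged as a light attack with a fixed combo count, then trigger an axe hit sound cue and the target's hit reaction.
; It also commits the ability and starts the cooldown display on the player UI.
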(event Ability|EventActivateAbility
  (|PlayMontageandWaitProxy "None" (Variables|Default|GetMontage%20to%20Play) 1.0 "None" true 1.0 0.0 false
    (:then
      (Utilities|FlowControl|Sequence
        (:then_0
          (|Damage))
        (:then_1
          (|UIUpdate))))
    (:OnCompleted
      (Ability|EndAbility :!label _label))
    (:OnBlendOut
      (goto _label))
    (:OnInterrupted
      (goto _label))
    (:OnCancelled
      (goto _label))))

(event Ability|EventOnEndAbility
  (params (bWasCancelled :type Boolean)))

(fn HandleApplyDamage
  (params (InPayload :type Gameplay%20Event%20Data%20Structure%20%28by%20ref%29))
  (bind _output_get (LocalVariables|SetCachedTargetActor (.Target (Utilities|Struct|BreakGameplayEventData InPayload))))
  (Class|CCreatureGameplayAbility|ApplyEffectSpecHandletoTarget _output_get (Class|CPlayerGameplayAbility|MakePlayerDamageEffectSpecHandle "/Game/Blueprint/Creature/Shared/GameplayEffect/GE_Shared_DealDamage.GE_Shared_DealDamage_C" (+ (Class|CPlayerCombatComponent|GetPlayerCurrentEquippedWeaponDamageatLevel (Class|CPlayerGameplayAbility|GetPlayerCombatComponentfromActorInfo) (Math|Conversions|ToFloat(Integer) (Ability|GetAbilityLevel))) 2.0) "(TagName=\"Player.SetByCaller.AttackType.Light\")" 4)
    (:Succesful
      (GameplayCue|ExecuteGameplayCue :GameplayCueTag "(TagName=\"GameplayCue.Sound.MeleeHit.Axe\")")
      (Ability|SendGameplayEventtoActor (LocalVariables|GetCachedTargetActor) "(TagName=\"Shared.Ability.HitReact\")" InPayload))))