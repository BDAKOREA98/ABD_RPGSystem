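; Player gameplay ability that plays the axe equip montage and ends when it finishes, blends out, or is interrupted or cancelled.
; On the axe equip gameplay event, it snaps the carried axe to the spine_Axe socket.
; HandleEquipWeapon would apply weapon data to anim layers, input mapping, granted abilities and UI, but its call is disconnected.
; The special-ability icon and cooldown updates are also unwired.
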(event Ability|EventActivateAbility
  (|PlayMontageandWaitProxy "None" "/Game/Creature/Player/Animation/Montage/Axe/AM_Player_Axe_Equip.AM_Player_Axe_Equip" 1.0 "None" true 1.0 0.0 false
    (:then
      (Ability|Tasks|WaitGameplayEvent "(TagName=\"Player.Event.Equip.Axe\")" 0
        (:EventReceived
          (Transformation|AttachComponentToComponent (Class|CPawnCombatComponent|GetCreatureCarriedWeaponbyTag (Class|CPlayerGameplayAbility|GetPlayerCombatComponentfromActorInfo) "(TagName=\"Player.Weapon.Axe\")") (Class|GameplayAbility|GetOwningComponentfromActorInfo) "spine_Axe" "SnapToTarget" "KeepRelative" "KeepWorld" true))))
    (:OnCompleted
      (Ability|EndAbility :!label _label))
    (:OnBlendOut
      (goto _label))
    (:OnInterrupted
      (goto _label))
    (:OnCancelled
      (goto _label))))

(event Ability|EventOnEndAbility
  (params (bWasCancelled :type Boolean)))

(fn HandleEquipWeapon
  (params (InWeaponToEquip :type C%20Player%20Weapon%20Object%20Reference))
  (LocalVariables|SetCachedPlayerWeaponData (Variables|/Script/ABD_RPGSystem.C_PlayerWeapon|GetPlayerWeaponData InWeaponToEquip))
  (Utilities|FlowControl|Sequence
    (:then_0
      (|ChangeAnim))
    (:then_1
      (|BindInput))
    (:then_2
      (|GiveabilitytoActor))
    (:then_3
      (|UIUpdate))))