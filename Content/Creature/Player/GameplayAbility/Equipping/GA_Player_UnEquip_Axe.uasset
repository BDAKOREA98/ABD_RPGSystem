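; Player gameplay ability that unequips the axe.
; It plays the unequip montage, clears the combat component's equipped weapon tag, then waits for the Player.Event.Unequip.Axe gameplay event to attach the axe to the spine_Axe socket.
; It then reverses the weapon setup from cached weapon data: unlinking the anim layer, removing the input mapping context and granted abilities, and refreshing weapon and ability-slot UI.
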(event Ability|EventActivateAbility
  (|PlayMontageandWaitProxy "None" "/Game/Creature/Player/Animation/Montage/Axe/AM_Player_Axe_Unequip.AM_Player_Axe_Unequip" 1.0 "None" true 1.0 0.0 false
    (:then
      (Variables|/Script/ABD_RPGSystem.C_PawnCombatComponent|SetCurrentEquippedWeaponTag (Class|CPlayerGameplayAbility|GetPlayerCombatComponentfromActorInfo) "")
      (Ability|Tasks|WaitGameplayEvent "(TagName=\"Player.Event.Unequip.Axe\")" 0
        (:EventReceived
          (Transformation|AttachComponentToComponent (Class|CPlayerCombatComponent|GetPlayerCarriedWeaponbyTag (Class|CPlayerGameplayAbility|GetPlayerCombatComponentfromActorInfo) "(TagName=\"Player.Weapon.Axe\")") (Class|GameplayAbility|GetOwningComponentfromActorInfo) "spine_Axe" "SnapToTarget" "KeepRelative" "KeepWorld" true)
          (CallFunction|HandlingUnequipWeapon (Class|CPlayerCombatComponent|GetPlayerCarriedWeaponbyTag (Class|CPlayerGameplayAbility|GetPlayerCombatComponentfromActorInfo) "(TagName=\"Player.Weapon.Axe\")")))))))

(event Ability|EventOnEndAbility
  (params (bWasCancelled :type Boolean)))

(fn HandlingUnequipWeapon
  (params (InWeaponData :type C%20Player%20Weapon%20Object%20Reference))
  (LocalVariables|SetCachedPlayerWeaponData (Variables|/Script/ABD_RPGSystem.C_PlayerWeapon|GetPlayerWeaponData InWeaponData))
  (Utilities|FlowControl|Sequence
    (:then_0
      (|ChangeAnim))
    (:then_1
      (|UnbindInput))
    (:then_2
      (|RemoveabilitytoActor))
    (:then_3
      (|UpdateUI))))