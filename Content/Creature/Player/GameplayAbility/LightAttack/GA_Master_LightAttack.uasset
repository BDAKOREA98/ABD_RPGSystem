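; Master player light-attack gameplay ability that plays a combo montage chain indexed by a counter.
; Each activation advances the counter, tagging JumpToFinisher before the last step so a tagged activation plays the finisher; a timer set on montage end resets both.
; MeleeHit events apply combo-aware damage, trigger a hit cue and reaction, and grant rage.
; WhileRageEvent is an empty hook fired behind a tag check.
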(event Custom|ResetAttackComboCount
  (Variables|Default|SetCurrentLightAttackComboCount 1)
  (Class|CFunctionLibrary|RemoveGameplayTagfromActorifFound (Class|CPlayerGameplayAbility|GetPlayerCharacterfromActorInfo) "(TagName=\"Player.Status.JumpToFinisher\")"))

(event Custom|WhileRageEvent)

(event Ability|EventActivateAbility
  (Utilities|Time|ClearandInvalidateTimerbyHandle (Variables|Default|GetComboCountResetTimer))
  (Class|CFunctionLibrary|DoesActorHaveTag (Class|CPlayerGameplayAbility|GetPlayerCharacterfromActorInfo) "(TagName=\"Player.Status.JumpToFinisher\")"
    (:YES
      (Variables|Default|SetCurrentLightAttackComboCount (Utilities|Map|Length (Variables|Default|GetAttackMoontages))))
    (:NO
      _))
  (Variables|Default|SetUsedComboCount (Variables|Default|GetCurrentLightAttackComboCount))
  (|PlayMontageandWaitProxy "None" (.Value (Utilities|Map|Find (Variables|Default|GetAttackMoontages) (Variables|Default|GetCurrentLightAttackComboCount))) 1.0 "None" true 1.0 0.0 false
    (:then
      (Utilities|FlowControl|Sequence
        (:then_0
          (|ApplyMeleeDamage))
        (:then_1
          (|HandleComboCount))
        (:then_2
          (Class|CFunctionLibrary|DoesActorHaveTag (Class|CPlayerGameplayAbility|GetPlayerCharacterfromActorInfo)
            (:YES
              (CallFunction|WhileRageEvent))))))
    (:OnCompleted
      (Ability|EndAbility :!label _label)
      (bind _returnvalue (Utilities|Time|SetTimerbyEvent (delegate Custom|ResetAttackComboCount) 0.0))
      (Variables|Default|SetComboCountResetTimer _returnvalue))
    (:OnBlendOut
      (goto _label))
    (:OnInterrupted
      (goto _label))
    (:OnCancelled
      (goto _label))))

(fn HandleApplyDamage
  (params (GameplayEventData :type Gameplay%20Event%20Data%20Structure%20%28by%20ref%29))
  (bind _output_get (LocalVariables|SetLocalTargetActor (.Target (Utilities|Struct|BreakGameplayEventData GameplayEventData))))
  (GameplayCue|ExecuteGameplayCue :GameplayCueTag (Variables|Default|GetWeaponHitSoundTag))
  (Class|CCreatureGameplayAbility|ApplyEffectSpecHandletoTarget _output_get (Class|CPlayerGameplayAbility|MakePlayerDamageEffectSpecHandle "/Game/Creature/Shared/GameplayEffect/GE_Shared_DealDamage.GE_Shared_DealDamage_C" (Class|CPlayerCombatComponent|GetPlayerCurrentEquippedWeaponDamageatLevel (Class|CPlayerGameplayAbility|GetPlayerCombatComponentfromActorInfo) (Math|Conversions|ToFloat(Integer) (Ability|GetAbilityLevel))) "(TagName=\"Player.SetByCaller.AttackType.Light\")" (Variables|Default|GetUsedComboCount))
    (:Succesful
      (Ability|SendGameplayEventtoActor (LocalVariables|GetLocalTargetActor) "(TagName=\"Shared.Event.HitReact\")" GameplayEventData)
      (Ability|ApplyGameplayEffectToOwner "/Game/Creature/Player/GameplayEffect/GE_Player_GainRage.GE_Player_GainRage_C" (Ability|GetAbilityLevel)))))